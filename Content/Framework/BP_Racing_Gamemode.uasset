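; Racing game mode that spawns the selected vehicle, runs the race clock and pays out a reward at the finish.
; The construction script maps the game instance's CurrentVehicle to DefaultPawnClass.
; Tick formats world game time into a minutes:seconds.centiseconds string until IsFinished is set.
; Once finished, it keeps stopping the vehicle's movement and, only once, adds random prize money to the game instance and saves it.
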(event EventBeginPlay)

(event EventTick
  (params (DeltaSeconds :type Float%20%28single-precision%29))
  (bind _returnvalue (Game|GetGameInstance))
  (bind _asgi_racing (Utilities|Casting|CastToGI_Racing _returnvalue))
  (if (Variables|Default|GetIsFinished)
    (Class|NavMovementComponent|StopMovementKeepPathing (Variables|/Script/ChaosVehicles.WheeledVehiclePawn|GetVehicleMovementComponent (.AsVehicle%20Pawn (Utilities|Casting|CastToVehiclePawn (Game|Player|GetPlayerPawn 0)))))
    (Utilities|FlowControl|DoOnce false
      (:Completed
        (bind _output_get (Variables|/Game/Framework/BP_PC_Racing.BP_PC_Racing_C|SetRandomMoney (.AsBP%20PC%20Racing (Utilities|Casting|CastToBP_PC_Racing (Game|GetPlayerController 0))) (Math|Random|RandomInteger 30000)))
        (Variables|/Game/Framework/GI_Racing.GI_Racing_C|SetMoney _asgi_racing (+ (Variables|/Game/Framework/GI_Racing.GI_Racing_C|GetMoney _asgi_racing) _output_get))
        (Default|SaveMoney _asgi_racing)))
    (else
      (Variables|Default|SetTime (Utilities|Time|GetTimeSeconds))
      (Utilities|FlowControl|Sequence
        (:then_0
          (if (== (Utilities|String|Len (Utilities|String|ToString(Integer) (Math|Integer|%(Integer) (Math|Conversions|ToInteger(Byte) (Class|KismetMathLibrary|ToInt64(Float) (Variables|Default|GetTime))) 60))) 1)
            (if (== (Utilities|String|Len (Utilities|String|ToString(Integer) (Math|Integer|%(Integer) (Math|Conversions|ToInteger(Byte) (Class|KismetMathLibrary|ToInt64(Float) (* (/ (Variables|Default|GetTime) 1.0) 1e+02))) 100))) 1)
              (Variables|Default|SetSTime (Utilities|String|Append (Utilities|String|ToString(Integer) (/ (Math|Conversions|ToInteger(Byte) (Class|KismetMathLibrary|ToInt64(Float) (Variables|Default|GetTime))) 60)) ":" (Utilities|String|Append "0" (Utilities|String|ToString(Integer) (Math|Integer|%(Integer) (Math|Conversions|ToInteger(Byte) (Class|KismetMathLibrary|ToInt64(Float) (Variables|Default|GetTime))) 60))) "." (Utilities|String|Append (Utilities|String|ToString(Integer) (Math|Integer|%(Integer) (Math|Conversions|ToInteger(Byte) (Class|KismetMathLibrary|ToInt64(Float) (* (/ (Variables|Default|GetTime) 1.0) 1e+02))) 100)) "0")))
              (else
                (Variables|Default|SetSTime (Utilities|String|Append (Utilities|String|ToString(Integer) (/ (Math|Conversions|ToInteger(Byte) (Class|KismetMathLibrary|ToInt64(Float) (Variables|Default|GetTime))) 60)) ":" (Utilities|String|Append "0" (Utilities|String|ToString(Integer) (Math|Integer|%(Integer) (Math|Conversions|ToInteger(Byte) (Class|KismetMathLibrary|ToInt64(Float) (Variables|Default|GetTime))) 60))) "." (Utilities|String|ToString(Integer) (Math|Integer|%(Integer) (Math|Conversions|ToInteger(Byte) (Class|KismetMathLibrary|ToInt64(Float) (* (/ (Variables|Default|GetTime) 1.0) 1e+02))) 100))))))
            (elif (== (Utilities|String|Len (Utilities|String|ToString(Integer) (Math|Integer|%(Integer) (Math|Conversions|ToInteger(Byte) (Class|KismetMathLibrary|ToInt64(Float) (* (/ (Variables|Default|GetTime) 1.0) 1e+02))) 100))) 1)
              (Variables|Default|SetSTime (Utilities|String|Append (Utilities|String|ToString(Integer) (/ (Math|Conversions|ToInteger(Byte) (Class|KismetMathLibrary|ToInt64(Float) (Variables|Default|GetTime))) 60)) ":" (Utilities|String|ToString(Integer) (Math|Integer|%(Integer) (Math|Conversions|ToInteger(Byte) (Class|KismetMathLibrary|ToInt64(Float) (Variables|Default|GetTime))) 60)) "." (Utilities|String|Append (Utilities|String|ToString(Integer) (Math|Integer|%(Integer) (Math|Conversions|ToInteger(Byte) (Class|KismetMathLibrary|ToInt64(Float) (* (/ (Variables|Default|GetTime) 1.0) 1e+02))) 100)) "0")))
              (else
                (Variables|Default|SetSTime (Utilities|String|Append (Utilities|String|ToString(Integer) (/ (Math|Conversions|ToInteger(Byte) (Class|KismetMathLibrary|ToInt64(Float) (Variables|Default|GetTime))) 60)) ":" (Utilities|String|ToString(Integer) (Math|Integer|%(Integer) (Math|Conversions|ToInteger(Byte) (Class|KismetMathLibrary|ToInt64(Float) (Variables|Default|GetTime))) 60)) "." (Utilities|String|ToString(Integer) (Math|Integer|%(Integer) (Math|Conversions|ToInteger(Byte) (Class|KismetMathLibrary|ToInt64(Float) (* (/ (Variables|Default|GetTime) 1.0) 1e+02))) 100))))))))))))

(fn ConstructionScript
  (switch Utilities|FlowControl|Switch|SwitchonVehicleList (Variables|/Game/Framework/GI_Racing.GI_Racing_C|GetCurrentVehicle (.AsGI%20Racing (Utilities|Casting|CastToGI_Racing (Game|GetGameInstance))))
    (:NewEnumerator0
      (Variables|Default|SetDefaultPawnClass "/Game/VehicleVarietyPack/Blueprints/SUV/BP_SUV.BP_SUV_C"))
    (:NewEnumerator1
      (Variables|Default|SetDefaultPawnClass "/Game/VehicleVarietyPack/Blueprints/Pickup/BP_Pickup.BP_Pickup_C"))
    (:NewEnumerator2
      (Variables|Default|SetDefaultPawnClass "/Game/VehicleVarietyPack/Blueprints/Truck/BP_Truck.BP_Truck_C"))
    (:NewEnumerator3
      (Variables|Default|SetDefaultPawnClass "/Game/VehicleVarietyPack/Blueprints/Hatchback/BP_Hatchback.BP_Hatchback_C"))
    (:NewEnumerator4
      (Variables|Default|SetDefaultPawnClass "/Game/VehicleVarietyVol2/Blueprints/BoxTruck/BoxTruck_VehicleConfig/BP_BoxTruck.BP_BoxTruck_C"))
    (:NewEnumerator5
      (Variables|Default|SetDefaultPawnClass "/Game/VehicleVarietyVol2/Blueprints/SUV/SUV_Config/BP_SUV_a.BP_SUV_a_C"))
    (:NewEnumerator6
      (Variables|Default|SetDefaultPawnClass "/Game/VehicleVarietyVol2/Blueprints/Campervan/Campervan_Config/BP_Campervan.BP_Campervan_C"))
    (:NewEnumerator7
      (Variables|Default|SetDefaultPawnClass "/Game/VehicleVarietyVol2/Blueprints/Sedan/Sedan_Config/BP_Sedan.BP_Sedan_C"))
    (:NewEnumerator8
      (Variables|Default|SetDefaultPawnClass "/Game/VehicleVarietyPack/Blueprints/SportsCar/BP_SportsCar.BP_SportsCar_C"))))