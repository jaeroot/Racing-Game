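; BP_PC_Racing is the racing player controller, which sets up the on-screen time widget and an Escape-key menu.
; BeginPlay creates WB_ESC as a hidden viewport widget and adds WB_Time to the viewport.
; Pressing Escape flips the IsOption flag to show or hide the menu and the mouse cursor together, without changing input mode or pause state.
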(event EventBeginPlay
  (bind _returnvalue (UserInterface|CreateWidget "/Game/WB/WB_ESC.WB_ESC_C" self))
  (bind _output_get (Variables|Default|SetOptionWidget _returnvalue))
  (UserInterface|Viewport|AddtoViewport _output_get 0)
  (Widget|SetVisibility _output_get "Hidden")
  (bind _returnvalue_2 (UserInterface|CreateWidget "/Game/WB/WB_Time.WB_Time_C" self))
  (UserInterface|Viewport|AddtoViewport _returnvalue_2 0))

(event EventTick
  (params (DeltaSeconds :type Float%20%28single-precision%29)))

(event Input|KeyboardEvents|Escape
  (params (Key :type Key%20Structure :default "None"))
  (bind _optionwidget (Variables|Default|GetOptionWidget))
  (:Pressed
    (if (Variables|Default|GetIsOption)
      (Variables|Default|SetbShowMouseCursor false)
      (Variables|Default|SetIsOption false)
      (Widget|SetVisibility _optionwidget "Hidden")
      (else
        (Variables|Default|SetbShowMouseCursor true)
        (Variables|Default|SetIsOption true)
        (Widget|SetVisibility _optionwidget "Visible")))))

(fn ConstructionScript)